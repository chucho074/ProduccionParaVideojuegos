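; Capture-the-flag base that owns a team's flag and tracks that team's points.
; When a character overlaps its sphere, an enemy picks up the flag if present, while an owning-team carrier scores a point.
; Scoring clears the carrier's flag and restores it at that player's enemy base.
; Pickup, scoring and reset run through Server-prefixed events, and the construction script sizes the sphere from a radius variable.
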(event OnComponentBeginOverlap(Sphere)
  (params (OverlappedComponent :type Primitive%20Component%20Object%20Reference) (OtherActor :type Actor%20Object%20Reference) (OtherComp :type Primitive%20Component%20Object%20Reference) (OtherBodyIndex :type Integer) (bFromSweep :type Boolean) (SweepResult :type Hit%20Result%20Structure%20%28by%20ref%29))
  (bind _asbp_character (Utilities|Casting|CastToBP_character OtherActor))
  (if (== (Variables|/Game/Blueprints/Personajes/BP_character.BP_character_C|GetTeam _asbp_character) (Variables|Default|GetOwnerTeam))
    (if (Variables|/Game/Blueprints/Personajes/BP_character.BP_character_C|GetisCarryingFlag _asbp_character)
      (CallFunction|ServerAddPoint)
      (CallFunction|ServerResetFlag _asbp_character))
    (elif (Variables|Default|GethasFlag)
      (CallFunction|ServerPlayerPickUpFlag _asbp_character))))

(event Custom|Server_Reset_Flag
  (params (Player :type BP%20Character%20Object%20Reference))
  (Variables|BP_flagBase_C|SethasFlag (Variables|/Game/Blueprints/Personajes/BP_character.BP_character_C|GetEnemyFlagBase Player) true)
  (Variables|/Game/Blueprints/Personajes/BP_character.BP_character_C|SetisCarryingFlag Player false))

(event Custom|Server_AddPoint
  (Variables|Default|SetteamPoints (+ (Variables|Default|GetteamPoints) 1)))

(event Custom|Server_Player_PickUp_Flag
  (params (Player :type BP%20Character%20Object%20Reference))
  (Variables|Default|SethasFlag false)
  (Variables|/Game/Blueprints/Personajes/BP_character.BP_character_C|SetisCarryingFlag Player true))

(fn ConstructionScript
  (Components|Sphere|SetSphereRadius (Variables|Default|GetSphere) (Variables|Default|GetRadiusValue) true))